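; An archived player pawn that moves forward and vertically from axis input and can grab and carry physics objects.
; Grab line-traces along the controller's forward vector for a physics body and passes it to a Physics Handle, whose target follows the control rotation every Tick until release.
; A Jump event applies a location-scaled impulse, and wall hits print the wall's name; several look, strafe and jump-toggle chains are left disconnected.
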(event OnComponentHit(collisionComponent)
  (params (HitComponent :type Primitive%20Component%20Object%20Reference) (OtherActor :type Actor%20Object%20Reference) (OtherComp :type Primitive%20Component%20Object%20Reference) (NormalImpulse :type Vector :default "0, 0, 0") (Hit :type Hit%20Result%20Structure%20%28by%20ref%29))
  (bind _asbp_wall (Utilities|Casting|CastToBP_Wall OtherActor))
  (Development|PrintString (Utilities|GetDisplayName _asbp_wall)))

(event Custom|Jump
  ;[1 1 1] Input movement
  (Utilities|NewMacro0))

(event EventTick
  (params (DeltaSeconds :type Float%20%28single-precision%29))
  ;[1 1 1] Set Handle Location and rotation
  (Class|PhysicsHandleComponent|SetTargetLocationandRotation (Variables|Default|GetPhysicsHandle) (+ (Transformation|GetActorLocation) (* (Math|Vector|GetForwardVector (Pawn|GetControlRotation :!class /Script/Engine.Pawn)) (Variables|Default|GetGrabLocation))) (Pawn|GetControlRotation :!class /Script/Engine.Pawn)))

(event Input|ActionEvents|InputActionGrab
  (params (Key :type Key%20Structure))
  (bind _self self)
  (bind _returnvalue (Transformation|GetActorLocation _self))
  ;[1 1 1] Grab Actor (Physics Actor)
  (:Pressed
    (bind (_outhit _returnvalue_2) (Collision|LineTraceForObjects _returnvalue (+ _returnvalue (* (Transformation|GetActorForwardVector (Game|GetPlayerController 0)) (Variables|Default|GetDistance))) (Utilities|Array|MakeArray "ObjectTypeQuery4") false 0 "ForDuration"))
    (if _returnvalue_2
      (Variables|Default|SetPhysicsObject (.HitComponent (Collision|BreakHitResult _outhit)))
      (Class|PhysicsHandleComponent|GrabComponentatLocation (Variables|Default|GetPhysicsHandle) (.HitComponent (Collision|BreakHitResult _outhit)) "None" (.Location (Collision|BreakHitResult _outhit)))))
  (:Released
    (Physics|Components|PhysicsHandle|ReleaseComponent (Variables|Default|GetPhysicsHandle))))

(event Input|ActionEvents|InputActionJump
  (params (Key :type Key%20Structure))
  ;[1 1 1] Input movement
)

(event Input|AxisEvents|InputAxisMoveForward
  (params (AxisValue :type Float%20%28single-precision%29))
  (bind _returnvalue (Pawn|GetController))
  (bind _returnvalue_2 (Transformation|GetActorForwardVector _returnvalue))
  ;[1 1 1] Input movement
  (Pawn|Input|AddMovementInput (Math|Vector|MakeVector (.x _returnvalue_2) (.y _returnvalue_2) 0.0) AxisValue true))

(event Input|AxisEvents|InputAxisJump
  (params (AxisValue :type Float%20%28single-precision%29))
  ;[1 1 1] Input movement
  (Pawn|Input|AddMovementInput (Math|Vector|MakeVector 0.0 0.0 AxisValue) 1.0 true))

(fn ConstructionScript)

(fn PrintFct
  (for _index (range (Variables|Default|Gethealth) 10)
    _)
  (Development|PrintString (Utilities|String|ToString(Integer) _index)))